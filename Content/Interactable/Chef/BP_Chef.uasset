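; BP_Chef is an interactable chef NPC that opens dialogue and unlocks weapons.
; Overlap with its collision by the first-person character toggles the prompt text, input and a nearby flag.
; Pressing Interact shows the cursor and one of three dialogue widgets chosen by the GameInstance's dialogue number, with the later two unlocking weapons 2 and 3.
; While the player is nearby, Tick turns the text using the controller's rotation.
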(event OnComponentBeginOverlap(ChefCollision)
  (params (OverlappedComponent :type Primitive%20Component%20Object%20Reference) (OtherActor :type Actor%20Object%20Reference) (OtherComp :type Primitive%20Component%20Object%20Reference) (OtherBodyIndex :type Integer) (bFromSweep :type Boolean) (SweepResult :type Hit%20Result%20Structure%20%28by%20ref%29))
  ;[1 1 1] Toggle Interact Text on overlap
  (Utilities|Casting|CastToFirstPersonCharacter OtherActor)
  (if (stale _bsuccess)
    (Rendering|SetVisibility (Variables|Default|GetChefText) true false)
    (Input|EnableInput (Game|GetPlayerController 0))
    (Variables|Default|SetIsPlayerNearby true)))

(event OnComponentEndOverlap(ChefCollision)
  (params (OverlappedComponent :type Primitive%20Component%20Object%20Reference) (OtherActor :type Actor%20Object%20Reference) (OtherComp :type Primitive%20Component%20Object%20Reference) (OtherBodyIndex :type Integer))
  ;[1 1 1] Toggle Interact Text on overlap
  (Utilities|Casting|CastToFirstPersonCharacter OtherActor)
  (if (stale _bsuccess)
    (Rendering|SetVisibility (Variables|Default|GetChefText) false false)
    (Input|DisableInput (Game|GetPlayerController 0))
    (Variables|Default|SetIsPlayerNearby false)))

(event EventTick
  (params (DeltaSeconds :type Float%20%28single-precision%29))
  (bind _cheftext (Variables|Default|GetChefText))
  (if (Variables|Default|GetIsPlayerNearby)
    ;[1 1 1] Make the text face the player
    (Transformation|SetWorldRotation _cheftext (.Rotation (Math|Transform|BreakTransform (Transformation|GetActorTransform (Game|GetPlayerController 0)))) false false)
    (Transformation|AddLocalRotation _cheftext "0,180.000000, 0" false false)))

(event Input|ActionEvents|InputActionInteract
  (params (Key :type Key%20Structure))
  ;[1 1 1] When you press the Interact ( E ) Key - Create the widget, add it to the viewport, then show the mouse cursor
  (:Pressed
    (if (Variables|Default|GetIsPlayerNearby)
      (bind _asmy_game_instance (Utilities|Casting|CastToMyGameInstance (Game|GetGameInstance)))
      (switch int (Variables|/Game/FirstPersonBP/Blueprints/MyGameInstance.MyGameInstance_C|GetChefDialogueNumber _asmy_game_instance)
        (:0
          (bind _returnvalue (UserInterface|CreateWidget "/Game/Interactable/Chef/DLG_Chef_0.DLG_Chef_0_C"))
          (UserInterface|Viewport|AddtoViewport _returnvalue 0))
        (:1
          (bind _returnvalue_2 (UserInterface|CreateWidget "/Game/Interactable/Chef/DLG_Chef_1.DLG_Chef_1_C"))
          (Variables|/Game/FirstPersonBP/Blueprints/MyGameInstance.MyGameInstance_C|SetWeapon2Unlocked _asmy_game_instance true)
          (UserInterface|Viewport|AddtoViewport _returnvalue_2 0))
        (:2
          (bind _returnvalue_3 (UserInterface|CreateWidget "/Game/Interactable/Chef/DLG_Chef_2.DLG_Chef_2_C"))
          (Variables|/Game/FirstPersonBP/Blueprints/MyGameInstance.MyGameInstance_C|SetWeapon3Unlocked _asmy_game_instance true)
          (UserInterface|Viewport|AddtoViewport _returnvalue_3 0)))
      (Variables|/Script/Engine.PlayerController|SetbShowMouseCursor (Game|GetPlayerController 0) true))))

(fn ConstructionScript)