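; BP_Key is a key pickup that the first-person character collects to record level progress.
; On overlap it adds its KeyType to the character's OwnedKeys, then for blue, red and both green types destroys itself and sets level completion flags on MyGameInstance.
; Blue, red and the second green key also advance the chef's dialogue number.
; The construction script picks the key's material from KeyType, with none assigned for the second green key.
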(event `self.Overlap.OnComponentBeginOverlap`
  (params (OverlappedComponent :type "PrimitiveComponent Object Reference") (OtherActor :type "Actor Object Reference") (OtherComp :type "PrimitiveComponent Object Reference") (OtherBodyIndex :type Integer) (bFromSweep :type Boolean) (SweepResult :type "HitResult Structure (by ref)"))
  (bind _keytype (`self.KeyType`))
  (bind _asfirst_person_character (cast `/Game/FirstPersonBP/Blueprints/FirstPersonCharacter` OtherActor))
  (`KismetArrayLibrary.Array_Add` (`/Game/FirstPersonBP/Blueprints/FirstPersonCharacter.OwnedKeys` _asfirst_person_character) _keytype)
  (switch `/Game/Interactable/EKeyType` _keytype
    (:`NewEnumerator1`
      (`self.K2_DestroyActor`)
      (bind _asmy_game_instance (cast `/Game/FirstPersonBP/Blueprints/MyGameInstance` (`GameplayStatics.GetGameInstance`)))
      (set `/Game/FirstPersonBP/Blueprints/MyGameInstance.LevelAComplete` true _asmy_game_instance)
      (set `/Game/FirstPersonBP/Blueprints/MyGameInstance.ChefDialogueNumber` 1 _asmy_game_instance))
    (:`NewEnumerator2`
      (`self.K2_DestroyActor`)
      (bind _asmy_game_instance_2 (cast `/Game/FirstPersonBP/Blueprints/MyGameInstance` (`GameplayStatics.GetGameInstance`)))
      (set `/Game/FirstPersonBP/Blueprints/MyGameInstance.LevelBComplete` true _asmy_game_instance_2)
      (set `/Game/FirstPersonBP/Blueprints/MyGameInstance.ChefDialogueNumber` 2 _asmy_game_instance_2))
    (:`NewEnumerator3`
      (`self.K2_DestroyActor`)
      (bind _asmy_game_instance_3 (cast `/Game/FirstPersonBP/Blueprints/MyGameInstance` (`GameplayStatics.GetGameInstance`)))
      (set `/Game/FirstPersonBP/Blueprints/MyGameInstance.LevelCHalfComplete` true _asmy_game_instance_3))
    (:`NewEnumerator4`
      (`self.K2_DestroyActor`)
      (bind _asmy_game_instance_4 (cast `/Game/FirstPersonBP/Blueprints/MyGameInstance` (`GameplayStatics.GetGameInstance`)))
      (set `/Game/FirstPersonBP/Blueprints/MyGameInstance.LevelCComplete` true _asmy_game_instance_4)
      (set `/Game/FirstPersonBP/Blueprints/MyGameInstance.ChefDialogueNumber` 3 _asmy_game_instance_4))))

(fn `UserConstructionScript`
  (`PrimitiveComponent.SetMaterial` (`self.Key`) 0 (select `/Game/Interactable/EKeyType` (`self.KeyType`) :`NewEnumerator0` "/Game/Interactable/M_BlackKey.M_BlackKey" :`NewEnumerator1` "/Game/Interactable/M_BlueKey.M_BlueKey" :`NewEnumerator2` "/Game/Interactable/M_RedKey.M_RedKey" :`NewEnumerator3` "/Game/Interactable/M_GreenKey.M_GreenKey" :!type "MaterialInterface Object Reference")))