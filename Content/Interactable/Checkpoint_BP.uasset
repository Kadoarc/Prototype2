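; Checkpoint actor that saves the player's location when its Trigger component is overlapped.
; The overlap reads player 0's FirstPersonCharacter location without checking which actor entered.
; It then loads the "Check" save slot, or creates a new SaveLocation object if none exists, writes the position into it and saves it back.
; Only saving happens here; nothing in this Blueprint restores the location.
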(event `self.Trigger.OnComponentBeginOverlap`
  (params (OverlappedComponent :type "PrimitiveComponent Object Reference") (OtherActor :type "Actor Object Reference") (OtherComp :type "PrimitiveComponent Object Reference") (OtherBodyIndex :type Integer) (bFromSweep :type Boolean) (SweepResult :type "HitResult Structure (by ref)"))
  (bind _playerloc (`self.PlayerLoc`))
  (`|ExecutionSequence`
    (:`then_0`
      (bind _asfirst_person_character (cast `/Game/FirstPersonBP/Blueprints/FirstPersonCharacter` (`GameplayStatics.GetPlayerCharacter` 0)))
      (set `self.PlayerLoc` (`self.K2_GetActorLocation` _asfirst_person_character)))
    (:`then_1`
      (bind _returnvalue (`GameplayStatics.DoesSaveGameExist` "Check"))
      (if _returnvalue
        (bind _returnvalue_2 (`GameplayStatics.LoadGameFromSlot` "Check"))
        (bind _assave_location (cast `/Game/Interactable/SaveLocation` _returnvalue_2))
        (set `/Game/Interactable/SaveLocation.PlayerLoc_S` _playerloc _assave_location)
        (`GameplayStatics.SaveGameToSlot` _assave_location "Check")
        (else
          (bind _returnvalue_3 (`GameplayStatics.CreateSaveGameObject` "/Game/Interactable/SaveLocation.SaveLocation_C"))
          (set `/Game/Interactable/SaveLocation.PlayerLoc_S` _playerloc _returnvalue_3)
          (`GameplayStatics.SaveGameToSlot` _returnvalue_3 "Check"))))))

(fn `UserConstructionScript`)